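; BP_Ennemy is a Skeleton King enemy that takes damage, shows its life and dies.
; On BeginPlay it loops an idle animation, records the starting LifePoint as MaxHealth and writes current/max to TextLife.
; DamageTaken, ignored once dead, plays a hit animation, subtracts damage and refreshes the text.
; At zero life or below it sets BIsDead, plays the death animation and destroys the actor after a short delay.
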(event `self.ReceiveBeginPlay`
  (bind _lifepoint (`self.LifePoint`))
  (`SkeletalMeshComponent.PlayAnimation` (`self.SkeletalMesh`) "/Game/SkeletonCrew/Skeleton_King/Animations/Skeleton_King_Idle_Loop.Skeleton_King_Idle_Loop" true)
  (bind _output_get (set `self.MaxHealth` _lifepoint))
  (`TextRenderComponent.K2_SetText` (`self.TextLife`) (`KismetTextLibrary.Conv_StringToText` (`KismetStringLibrary.Concat_StrStr` (`KismetStringLibrary.Conv_DoubleToString` _lifepoint) "/" (`KismetStringLibrary.Conv_DoubleToString` _output_get)))))

(event `/Game/Blueprint/BPI_Damage.DamageTaken`
  (params (DamageDo :type "Float (double-precision)"))
  (if (not (`self.b_IsDead`))
    (`SkeletalMeshComponent.PlayAnimation` (`self.SkeletalMesh`) "/Game/SkeletonCrew/Skeleton_King/Animations/Skeleton_King_Hit_Back.Skeleton_King_Hit_Back" false)
    (set `self.LifePoint` (- (`self.LifePoint`) DamageDo))
    (`TextRenderComponent.K2_SetText` (`self.TextLife`) (`KismetTextLibrary.Conv_StringToText` (`KismetStringLibrary.Concat_StrStr` (`KismetStringLibrary.Conv_DoubleToString` (`self.LifePoint`)) "/" (`KismetStringLibrary.Conv_DoubleToString` (`self.MaxHealth`)))))
    (if (<= (`self.LifePoint`) 0.0)
      (set `self.b_IsDead` true)
      (`SkeletalMeshComponent.PlayAnimation` (`self.SkeletalMesh`) "/Game/SkeletonCrew/Skeleton_King/Animations/Skeleton_King_Death.Skeleton_King_Death" false)
      (`KismetSystemLibrary.Delay` 4.0)
      (`self.K2_DestroyActor`))))

(fn `UserConstructionScript`)